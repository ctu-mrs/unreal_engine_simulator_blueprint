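; BP_GetIsolatorLocation exports the positions of tower insulator markers to a CSV file when play begins.
; It gathers static mesh components tagged "insulator_marker" on all BP_TowerD and BP_TowerA actors.
; Each position gets a fixed Z offset, becomes relative to the PlayerStart, and is converted to right-handed meters by scaling and flipping Y.
; WriteGateTransformToCsv saves these with tower names and zero headings, and the result is printed.
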(event EventBeginPlay
  (bind _returnvalue (Actor|GetActorOfClass "/Script/Engine.PlayerStart"))
  (bind _outactors (Actor|GetAllActorsOfClass "/Game/Worlds/EletricTowers/TransmissionTowers/Blueprints/BP_Tower-D.BP_Tower-D_C"))
  (for _array_element _outactors
    (for _array_element_2 (Actor|GetComponentsbyTag _array_element "/Script/Engine.StaticMeshComponent" "insulator_marker")
      ;[1 1 1] Transformation from UE coord to Right-Hand cordinates
      (Utilities|Array|Add (Variables|Default|Getposition%20to%20print) (/ (- (+ (.location (Transformation|GetWorldTransform _array_element_2)) "0.000000,0.000000,92.120000") (Transformation|GetActorLocation _returnvalue)) "100.000000,-100.000000,100.000000"))
      (Utilities|Array|Add (Variables|Default|Getnames%20to%20print) (Utilities|GetDisplayName _array_element))
      (Utilities|Array|Add (Variables|Default|Getheading%20to%20print) 0.0)))
  (bind _outactors_2 (Actor|GetAllActorsOfClass "/Game/Worlds/EletricTowers/TransmissionTowers/Blueprints/BP_Tower-A.BP_Tower-A_C"))
  (for _array_element_3 _outactors_2
    (for _array_element_4 (Actor|GetComponentsbyTag _array_element_3 "/Script/Engine.StaticMeshComponent" "insulator_marker")
      (Utilities|Array|Add (Variables|Default|Getposition%20to%20print) (/ (- (+ (.location (Transformation|GetWorldTransform _array_element_4)) "0.000000,0.000000,92.120000") (Transformation|GetActorLocation _returnvalue)) "100.000000,-100.000000,100.000000"))
      (Utilities|Array|Add (Variables|Default|Getnames%20to%20print) (Utilities|GetDisplayName _array_element_3))
      (Utilities|Array|Add (Variables|Default|Getheading%20to%20print) 0.0)))
  (bind _outstring (Class|BlueprintUtils|WriteGateTransformtoCsv "Insulators_Position" (Variables|Default|Getnames%20to%20print) (Variables|Default|Getposition%20to%20print) (Variables|Default|Getheading%20to%20print)))
  (Development|PrintString _outstring))

(fn ConstructionScript)